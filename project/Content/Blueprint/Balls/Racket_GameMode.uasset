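; Game mode for a multiplayer racket game that spawns and possesses a racket pawn for each player who joins.
; On PostLogin, the authority spawns a RacketPlayer_Blueprint3 at a player start and has the new controller possess it.
; FindPlayerStart is overridden to pick from all PlayerStart actors by current player count, giving each successive player the next start without checking occupancy or bounds.
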(event `self.K2_PostLogin`
  (params (NewPlayer :type "PlayerController Object Reference"))
  ;[1 1 1] When a player joins game
  (`/Engine/EditorBlueprintResources/ActorMacros.Switch Has Authority`
    (:`Authority`
      (bind _returnvalue (`|SpawnActorFromClass` "/Game/Blueprint/Balls/RacketPlayer_Blueprint3.RacketPlayer_Blueprint3_C" (`self.GetTransform` (`self.K2_FindPlayerStart` null)) "AdjustIfPossibleButAlwaysSpawn" "OverrideRootScale" null null))
      (`Controller.Possess` NewPlayer _returnvalue))))

(fn `FindPlayerStart`
  (params (Player :type "Controller Object Reference") (IncomingName :type String))
  (returns (ReturnValue :type "Actor Object Reference"))
  ;[1 1 1] Return unused Player Start
  (bind _returnvalue (`self.GetNumPlayers`))
  (bind _outactors (`GameplayStatics.GetAllActorsOfClass` "/Script/Engine.PlayerStart"))
  (return (`|GetArrayItem` _outactors (- _returnvalue 1))))

(fn `UserConstructionScript`)