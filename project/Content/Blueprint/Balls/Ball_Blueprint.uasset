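; Ball actor Blueprint with a physics-simulated collision sphere, launched and redirected through velocity events.
; Direction and random-speed events compute velocities from the ball's min/max speeds and feed SetVelocity, which a DoOnce locks for half a second.
; The first hit while simulating sets IsLaunched, and destruction spawns a randomly rotated emitter.
; Tick is empty; speed clamping, dead-ball blinking and respawn logic are disconnected, and passed colors go unused.
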(event `self.ReceiveTick`
  (params (DeltaSeconds :type "Float (single-precision)"))
  ;[0 0.02625 0.13] Tick
)

(event `Enable Physics Simulation`
  (bind _collisionsphere (`self.CollisionSphere`))
  ;[0.16 0 0] Custom Events
  (`PrimitiveComponent.SetSimulatePhysics` _collisionsphere true)
  (`PrimitiveComponent.SetAllPhysicsLinearVelocity` _collisionsphere (0.0 0.0 0.0) false))

(event `Set Velocity`
  (params (`New Velocity` :type "Vector Structure") (`New Color` :type "LinearColor Structure"))
  ;[0.16 0 0] Custom Events
  (`/Engine/EditorBlueprintResources/StandardMacros.DoOnce` false :!label _label
    (:`Completed`
      (`PrimitiveComponent.SetAllPhysicsLinearVelocity` (`self.CollisionSphere`) `New Velocity` false)
      (`KismetSystemLibrary.Delay` 0.5)
      (goto _label :!via `Reset`))))

(event `Set Movement Direction`
  (params (`New Direction` :type "Vector Structure") (`New Color` :type "LinearColor Structure"))
  ;[0.16 0 0] Custom Events
  (`self. Set Velocity` (* (`KismetMathLibrary.Normal` `New Direction`) (`KismetMathLibrary.FClamp` (`KismetMathLibrary.VSize` (`self.GetVelocity`)) (`self.Ball Min Speed`) (`self.Ball Max Speed`))) `New Color`))

(event `Set Random Velocity`
  (params (`New Direction` :type "Vector Structure") (`Min Speed Ratio` :type "Float (double-precision)" :default 0.5) (`New Color` :type "LinearColor Structure"))
  ;[0.16 0 0] Custom Events
  (`self. Set Velocity` (* (`KismetMathLibrary.Normal` `New Direction`) (* (`KismetMathLibrary.RandomFloatInRange` `Min Speed Ratio` 1.0) (`self.Ball Max Speed`))) `New Color`))

(event `self.CollisionSphere.OnComponentHit`
  (params (HitComponent :type "PrimitiveComponent Object Reference") (OtherActor :type "Actor Object Reference") (OtherComp :type "PrimitiveComponent Object Reference") (NormalImpulse :type "Vector Structure") (Hit :type "HitResult Structure (by ref)"))
  ;[0.19 0.117 0] Hit
  (if (`SceneComponent.IsSimulatingPhysics` (`self.CollisionSphere`) "None")
    (`/Engine/EditorBlueprintResources/StandardMacros.DoOnce` false
      (:`Completed`
        (set `self.Is Launched ?` true)))))

(event `self.ReceiveDestroyed`
  ;[1 0 0.4007] Destoyed
  (`GameplayStatics.SpawnEmitterAtLocation` null (`self.K2_GetActorLocation`) (`KismetMathLibrary.RandomRotator` true)))

(fn `UserConstructionScript`)