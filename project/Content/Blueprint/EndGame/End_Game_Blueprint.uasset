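; End-game screen actor that shows the winner, scores and heart-rate history for two players through a widget component.
; Events forward score updates, timed heart-rate samples and the winner to End_Game_Widget through a cast helper.
; Each heart-rate sample reads both players' values from Main_GameState.
; EndGame makes the whole component hierarchy visible, and SceneReset hides it again.
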(event `Scene Reset`
  (`SceneComponent.SetVisibility` (`self.DefaultSceneRoot`) false true))

(event `Score Updated`
  (params (`Player ID` :type Integer) (Score :type Integer))
  (bind _endgame (`self.Get End Game Widget`)
    (:`is Valid`
      (`/Game/Blueprint/EndGame/End_Game_Widget.Set Scores Text` _endgame `Player ID` Score))))

(event `Add HR Datapoint`
  (params (Time :type Integer))
  (bind _endgame (`self.Get End Game Widget`)
    (:`is Valid`
      (for _index (range 2)
        (bind _heartrate (`/Game/Main_GameState.Get HeartRate` (cast `/Game/Main_GameState` (`GameplayStatics.GetGameState`) :!pure true) _index))
        (`/Game/Blueprint/EndGame/End_Game_Widget.Add HR Datapoint` _endgame _index Time _heartrate)))))

(event `End Game`
  (params (Winner :type Boolean))
  (bind _endgame (`self.Get End Game Widget`)
    (:`is Valid`
      (`/Game/Blueprint/EndGame/End_Game_Widget.End Game` _endgame Winner)
      (`SceneComponent.SetVisibility` (`self.DefaultSceneRoot`) true true))))

(fn `UserConstructionScript`)