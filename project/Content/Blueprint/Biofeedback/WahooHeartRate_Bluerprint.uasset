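; Wahoo heart-rate biofeedback Blueprint that exchanges data with a local socket server.
; On BeginPlay, if it has ownership, it connects to localhost and retries whenever the connection drops.
; Each incoming message's first byte becomes the heart rate exposed by GetHeartRate.
; LogGameEvent calls its parent, then sends a start or non-start code back over the same connection.
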(event `self.ReceiveBeginPlay`
  (if (`self.Has Ownership`) :!label _label
    (bind _connectionid (`self.Connect` "127.0.0.1" 27015 (delegate `Disconnected_1`) (delegate `Connected_1`) (delegate `ReceivedMessage_1`)))
    (set `self.Connection ID` _connectionid)))

(event `Disconnected_1`
  (params (ConnectionId :type Integer))
  (goto _label))

(event `Connected_1`
  (params (ConnectionId :type Integer)))

(event `ReceivedMessage_1`
  (params (ConnectionId :type Integer) (Message :type "Array of Byte (by ref)"))
  (bind _returnvalue (`self.Message_ReadByte` Message))
  (set `self.hr` (`KismetMathLibrary.Conv_ByteToInt` _returnvalue)))

(event `self.Log Game Event`
  (params (`Start Event` :type Boolean))
  (`parent.Log Game Event` `Start Event`)
  (`self.SendData` (`self.Connection ID`) (`self.Conv_IntToBytes` (`KismetMathLibrary.SelectInt` 1 2 `Start Event`)))
  (`KismetSystemLibrary.PrintString` "Send Game Event to Wahoo"))

(fn `Get Heart Rate`
  (returns (HR :type Integer))
  (return (`self.HR`)))

(fn `UserConstructionScript`
  (`parent.UserConstructionScript`))