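; Two-player floor thermometer display that shows each player's score, heartbeat and green, yellow and red side warning lights around a movable center.
; Dynamic material instances drive the floor, player bases and lights, with alternating timers flashing the red lights.
; A looping timer eases displayed scores and center offset, repositioning lights as the center shifts.
; Heart rate sets timeline play rates for the pulse effect; numpad keys send debug changes through the GameMode.
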(event `self.ReceiveBeginPlay`
  ;[1 1 1] Initialization
  (`|ExecutionSequence`
    (:`then_0`
      (bind _returnvalue (`PrimitiveComponent.CreateDynamicMaterialInstance` (`self.Floor`) 0 "/Game/Assets/Thermometer/Thermometer_Material_v3.Thermometer_Material_v3" "None"))
      (bind _output_get (set `self.Thermometer Material` _returnvalue))
      (`MaterialInstanceDynamic.SetVectorParameterValue` _output_get "Player1 Color" (`KismetMathLibrary.Conv_ColorToLinearColor` (`self.Player 1 Color`)))
      (`MaterialInstanceDynamic.SetVectorParameterValue` _output_get "Player2 Color" (`KismetMathLibrary.Conv_ColorToLinearColor` (`self.Player 2 Color`)))
      (`MaterialInstanceDynamic.SetVectorParameterValue` _output_get "Base Color" (`KismetMathLibrary.Conv_ColorToLinearColor` (`self.Base Color`)))
      (`MaterialInstanceDynamic.SetScalarParameterValue` _output_get "Player Zone Percentage" (`self.GetPlayerZonePercentage`)))
    (:`then_1`
      (bind _returnvalue_2 (`PrimitiveComponent.CreateDynamicMaterialInstance` (`self.Player 1 Base`) 0 "/Game/Assets/Thermometer/ThermometerEnd_Material.ThermometerEnd_Material" "None"))
      (bind _output_get_2 (set `self.Base 1 Material` _returnvalue_2))
      (`MaterialInstanceDynamic.SetVectorParameterValue` _output_get_2 "Player Color" (`KismetMathLibrary.Conv_ColorToLinearColor` (`self.Player 1 Color`)))
      (`MaterialInstanceDynamic.SetVectorParameterValue` _output_get_2 "Base Color" (`KismetMathLibrary.Conv_ColorToLinearColor` (`self.Base Color`))))
    (:`then_2`
      (bind _returnvalue_3 (`PrimitiveComponent.CreateDynamicMaterialInstance` (`self.Player 2 Base`) 0 "/Game/Assets/Thermometer/ThermometerEnd_Material.ThermometerEnd_Material" "None"))
      (bind _output_get_3 (set `self.Base 2 Material` _returnvalue_3))
      (`MaterialInstanceDynamic.SetVectorParameterValue` _output_get_3 "Player Color" (`KismetMathLibrary.Conv_ColorToLinearColor` (`self.Player 2 Color`)))
      (`MaterialInstanceDynamic.SetVectorParameterValue` _output_get_3 "Base Color" (`KismetMathLibrary.Conv_ColorToLinearColor` (`self.Base Color`))))
    (:`then_3`
      (`self.Colour Side Lights`)
      (`self.Flash Open`)
      (`self.Start Smooth Score Update`))
    (:`then_4`
      (`self.Enable Keyboard`))))

(event `Colour Side Lights`
  ;[1 1 1] Sets the colors of each of the side lights
  (`|ExecutionSequence`
    (:`then_0`
      (bind _returnvalue (`PrimitiveComponent.CreateDynamicMaterialInstance` (`self.P1_side_green`) 0 "/Game/Assets/Thermometer/side_light_material.side_light_material" "None"))
      (bind _output_get (set `self.P1 Side Green Material` _returnvalue))
      (`MaterialInstanceDynamic.SetVectorParameterValue` _output_get "Color" (`KismetMathLibrary.Conv_ColorToLinearColor` (`self.OK Color`))))
    (:`then_1`
      (bind _returnvalue_2 (`PrimitiveComponent.CreateDynamicMaterialInstance` (`self.P1_side_yellow`) 0 "/Game/Assets/Thermometer/side_light_material.side_light_material" "None"))
      (bind _output_get_2 (set `self.P1 Side Yellow Material` _returnvalue_2))
      (`MaterialInstanceDynamic.SetVectorParameterValue` _output_get_2 "Color" (`KismetMathLibrary.Conv_ColorToLinearColor` (`self.Warning Color`))))
    (:`then_2`
      (bind _returnvalue_3 (`PrimitiveComponent.CreateDynamicMaterialInstance` (`self.P1_side_red`) 0 "/Game/Assets/Thermometer/side_light_material.side_light_material" "None"))
      (bind _output_get_3 (set `self.P1 Side Red Material` _returnvalue_3))
      (`MaterialInstanceDynamic.SetVectorParameterValue` _output_get_3 "Color" (`KismetMathLibrary.Conv_ColorToLinearColor` (`self.Alert Color`))))
    (:`then_3`
      (bind _returnvalue_4 (`PrimitiveComponent.CreateDynamicMaterialInstance` (`self.P2_side_green`) 0 "/Game/Assets/Thermometer/side_light_material.side_light_material" "None"))
      (bind _output_get_4 (set `self.P2 Side Green Material` _returnvalue_4))
      (`MaterialInstanceDynamic.SetVectorParameterValue` _output_get_4 "Color" (`KismetMathLibrary.Conv_ColorToLinearColor` (`self.OK Color`))))
    (:`then_4`
      (bind _returnvalue_5 (`PrimitiveComponent.CreateDynamicMaterialInstance` (`self.P2_side_yellow`) 0 "/Game/Assets/Thermometer/side_light_material.side_light_material" "None"))
      (bind _output_get_5 (set `self.P2 Side Yellow Material` _returnvalue_5))
      (`MaterialInstanceDynamic.SetVectorParameterValue` _output_get_5 "Color" (`KismetMathLibrary.Conv_ColorToLinearColor` (`self.Warning Color`))))
    (:`then_5`
      (bind _returnvalue_6 (`PrimitiveComponent.CreateDynamicMaterialInstance` (`self.P2_side_red`) 0 "/Game/Assets/Thermometer/side_light_material.side_light_material" "None"))
      (bind _output_get_6 (set `self.P2 Side Red Material` _returnvalue_6))
      (`MaterialInstanceDynamic.SetVectorParameterValue` _output_get_6 "Color" (`KismetMathLibrary.Conv_ColorToLinearColor` (`self.Alert Color`))))))

(event `Rescale Floor Material`
  (bind _percentage (`self.GetPlayerZonePercentage`))
  (bind _p2_side_red (`self.P2_side_red`))
  (bind _p2_side_yellow (`self.P2_side_yellow`))
  (bind _p1_side_red (`self.P1_side_red`))
  (bind _p1_side_green (`self.P1_side_green`))
  (bind _p2_side_green (`self.P2_side_green`))
  (bind _p1_side_yellow (`self.P1_side_yellow`))
  (bind _player_2_base (`self.Player 2 Base`))
  (bind _player_1_base (`self.Player 1 Base`))
  (bind _z (.z (`SceneComponent.K2_GetComponentScale` _p2_side_red)))
  (bind _z_2 (.z (`SceneComponent.K2_GetComponentScale` _p2_side_yellow)))
  (bind _z_3 (.z (`SceneComponent.K2_GetComponentScale` _p1_side_red)))
  (bind _z_4 (.z (`SceneComponent.K2_GetComponentScale` _p1_side_green)))
  (bind _z_5 (.z (`SceneComponent.K2_GetComponentScale` _p2_side_green)))
  (bind _z_6 (.z (`SceneComponent.K2_GetComponentScale` _p1_side_yellow)))
  (bind _returnvalue (* (- 1.0 (/ _percentage 2.0)) (* 50 (.y (`SceneComponent.K2_GetComponentScale` (`self.Floor`))))))
  (bind _returnvalue_2 (`KismetMathLibrary.MakeVector` 0.0 _returnvalue 0.1))
  (bind _returnvalue_3 (`KismetMathLibrary.MakeVector` 0.0 (* _returnvalue -1.0) 0.1))
  ;[1 1 1] Startup sequence
  (`self.Light PositionUpdate`)
  (`MaterialInstanceDynamic.SetScalarParameterValue` (`self.Thermometer Material`) "Player Zone Percentage" _percentage)
  (`SceneComponent.SetWorldScale3D` _player_1_base (1.0 1.0 1.0))
  (`SceneComponent.K2_SetWorldLocation` _player_1_base _returnvalue_2 false false)
  (message `/Game/GameModeInterface.Update Player Position` (`GameplayStatics.GetGameMode`) 0 (+ _returnvalue_2 (0.0 0.0 0.9)))
  (`SceneComponent.SetWorldScale3D` _player_2_base (1.0 1.0 1.0))
  (`SceneComponent.K2_SetWorldLocation` _player_2_base _returnvalue_3 false false)
  (message `/Game/GameModeInterface.Update Player Position` (`GameplayStatics.GetGameMode`) 1 (+ _returnvalue_3 (0.0 0.0 0.9)))
  (`|ExecutionSequence`
    (:`then_0`
      (`SceneComponent.SetWorldScale3D` _p1_side_green (`KismetMathLibrary.MakeVector` (.x (`SceneComponent.K2_GetComponentScale` _p1_side_green)) _z_4 _z_4)))
    (:`then_1`
      (`SceneComponent.SetWorldScale3D` _p2_side_green (`KismetMathLibrary.MakeVector` (.x (`SceneComponent.K2_GetComponentScale` _p2_side_green)) _z_5 _z_5)))
    (:`then_2`
      (`SceneComponent.SetWorldScale3D` _p1_side_yellow (`KismetMathLibrary.MakeVector` (.x (`SceneComponent.K2_GetComponentScale` _p1_side_yellow)) _z_6 _z_6)))
    (:`then_3`
      (`SceneComponent.SetWorldScale3D` _p2_side_yellow (`KismetMathLibrary.MakeVector` (.x (`SceneComponent.K2_GetComponentScale` _p2_side_yellow)) _z_2 _z_2)))
    (:`then_4`
      (`SceneComponent.SetWorldScale3D` _p1_side_red (`KismetMathLibrary.MakeVector` (.x (`SceneComponent.K2_GetComponentScale` _p1_side_red)) _z_3 _z_3)))
    (:`then_5`
      (`SceneComponent.SetWorldScale3D` _p2_side_red (`KismetMathLibrary.MakeVector` (.x (`SceneComponent.K2_GetComponentScale` _p2_side_red)) _z _z)))))

(event `Update Player Heart Rate`
  (params (ID :type Integer) (`Heart Rate` :type Integer))
  (bind _returnvalue (/ (`KismetMathLibrary.Conv_IntToDouble` `Heart Rate`) 60.0))
  ;[1 1 1] Update Display Variables
  (switch `int` ID
    (:`0`
      (`TimelineComponent.SetPlayRate` (`self.Timeline Player1`) _returnvalue))
    (:`1`
      (`TimelineComponent.SetPlayRate` (`self.Timeline Player2`) _returnvalue))))

(event `Lightup Side Indicators`
  (bind _score (`self.Get Score` (`self.Player1`)))
  ;[1 1 1] Startup sequence
  (`|ExecutionSequence`
    (:`then_0`
      (if (and (>= _score (`self.Green Light Offset`)) (not (`SceneComponent.IsVisible` (`self.Green Lights`))))
        (`SceneComponent.SetVisibility` (`self.Green Lights`) true true)
        (`self.Check Light Status` true :!label _label)
        (`self.Check Light Status` false)))
    (:`then_1`
      (if (and (>= _score (`self.Yellow Light Offset`)) (not (`SceneComponent.IsVisible` (`self.Yellow Lights`))))
        (`SceneComponent.SetVisibility` (`self.Yellow Lights`) true true)
        (goto _label)))
    (:`then_2`
      (if (and (>= _score (`self.Red Light Offset`)) (not (`SceneComponent.IsVisible` (`self.Red Lights`))))
        (`SceneComponent.SetVisibility` (`self.Red Lights`) true true)))))

(event `Light PositionUpdate`
  ;[1 1 1] Updates the location of the side indicators
  (`|ExecutionSequence` :!label _label_2
    (:`then_0`
      (`self.Place Light` (`self.Green Light Offset`) true (`self.P1_side_green`)))
    (:`then_1`
      (`self.Place Light` (`self.Yellow Light Offset`) true (`self.P1_side_yellow`)))
    (:`then_2`
      (`self.Place Light` (`self.Red Light Offset`) true (`self.P1_side_red`)))
    (:`then_3`
      (`self.Place Light` (`self.Green Light Offset`) false (`self.P2_side_green`)))
    (:`then_4`
      (`self.Place Light` (`self.Yellow Light Offset`) false (`self.P2_side_yellow`)))
    (:`then_5`
      (`self.Place Light` (`self.Red Light Offset`) false (`self.P2_side_red`)))))

(event `Light Position Update Multi`
  ;[1 1 1] Updates the location of the side indicators
  (goto _label_2))

(event `Key|NumPadSeven`
  (params (Key :type "Key Structure"))
  ;[1 1 1] Key shortcuts for development purposes
  (:`Pressed`
    (message `/Game/GameModeInterface.Set Player Score` (`GameplayStatics.GetGameMode`) 0 (+ (`self.Get Score` (`self.Player1`)) 0.05))))

(event `Key|NumPadOne`
  (params (Key :type "Key Structure"))
  ;[1 1 1] Key shortcuts for development purposes
  (:`Pressed`
    (message `/Game/GameModeInterface.Set Player Score` (`GameplayStatics.GetGameMode`) 0 (- (`self.Get Score` (`self.Player1`)) 0.05))))

(event `Key|NumPadThree`
  (params (Key :type "Key Structure"))
  ;[1 1 1] Key shortcuts for development purposes
  (:`Pressed`
    (message `/Game/GameModeInterface.Set Player Score` (`GameplayStatics.GetGameMode`) 1 (- (`self.Get Score` (`self.Player2`)) 0.05))))

(event `Key|NumPadNine`
  (params (Key :type "Key Structure"))
  ;[1 1 1] Key shortcuts for development purposes
  (:`Pressed`
    (message `/Game/GameModeInterface.Set Player Score` (`GameplayStatics.GetGameMode`) 1 (+ (`self.Get Score` (`self.Player2`)) 0.05))))

(event `Flash Open`
  (bind _red_light_offset (`self.Red Light Offset`))
  ;[1 1 1] Side Light Controller
  (bind _returnvalue (`KismetSystemLibrary.K2_SetTimerDelegate` (delegate `Flash Close`) 0.1))
  (set `self.Player Alert Timer` _returnvalue)
  (`|ExecutionSequence`
    (:`then_0`
      (bind _required_score (`self.Has Required Score To Open Light` _red_light_offset true))
      (`MaterialInstanceDynamic.SetScalarParameterValue` (`self.P1 Side Red Material`) "Intensity" (`KismetMathLibrary.Conv_BoolToDouble` _required_score)))
    (:`then_1`
      (bind _required_score_2 (`self.Has Required Score To Open Light` _red_light_offset))
      (`MaterialInstanceDynamic.SetScalarParameterValue` (`self.P2 Side Red Material`) "Intensity" (`KismetMathLibrary.Conv_BoolToDouble` _required_score_2)))))

(event `Key|NumPadFour`
  (params (Key :type "Key Structure"))
  ;[1 1 1] Key shortcuts for development purposes
  (:`Pressed`
    (message `/Game/GameModeInterface.Set Center Offset` (`GameplayStatics.GetGameMode`) (+ (`self.Center Offset`) 0.05))))

(event `Key|NumPadSix`
  (params (Key :type "Key Structure"))
  ;[1 1 1] Key shortcuts for development purposes
  (:`Pressed`
    (message `/Game/GameModeInterface.Set Center Offset` (`GameplayStatics.GetGameMode`) (- (`self.Center Offset`) 0.05))))

(event `Enable Keyboard`
  ;[1 1 1] Key shortcuts for development purposes
  (`self.EnableInput` (`GameplayStatics.GetPlayerController` 0)))

(event `Check Light Status`
  (params (`Is Player1` :type Boolean))
  (bind _green_light_offset (`self.Green Light Offset`))
  (bind _yellow_light_offset (`self.Yellow Light Offset`))
  ;[1 1 1] Side Light Controller
  (if `Is Player1`
    (bind _required_score (`self.Has Required Score To Open Light` _green_light_offset true))
    (`MaterialInstanceDynamic.SetScalarParameterValue` (`self.P1 Side Green Material`) "Intensity" (`KismetMathLibrary.Conv_BoolToDouble` _required_score))
    (bind _required_score_2 (`self.Has Required Score To Open Light` _yellow_light_offset true))
    (`MaterialInstanceDynamic.SetScalarParameterValue` (`self.P1 Side Yellow Material`) "Intensity" (`KismetMathLibrary.Conv_BoolToDouble` _required_score_2))
    (else
      (bind _required_score_3 (`self.Has Required Score To Open Light` _green_light_offset))
      (`MaterialInstanceDynamic.SetScalarParameterValue` (`self.P2 Side Green Material`) "Intensity" (`KismetMathLibrary.Conv_BoolToDouble` _required_score_3))
      (bind _required_score_4 (`self.Has Required Score To Open Light` _yellow_light_offset))
      (`MaterialInstanceDynamic.SetScalarParameterValue` (`self.P2 Side Yellow Material`) "Intensity" (`KismetMathLibrary.Conv_BoolToDouble` _required_score_4)))))

(event `Flash Close`
  ;[1 1 1] Side Light Controller
  (bind _returnvalue (`KismetSystemLibrary.K2_SetTimerDelegate` (delegate `Flash Open`) 0.1))
  (set `self.Player Alert Timer` _returnvalue)
  (`|ExecutionSequence`
    (:`then_0`
      (`MaterialInstanceDynamic.SetScalarParameterValue` (`self.P1 Side Red Material`) "Intensity" 0.0))
    (:`then_1`
      (`MaterialInstanceDynamic.SetScalarParameterValue` (`self.P2 Side Red Material`) "Intensity" 0.0))))

(event `Start Smooth Score Update`
  ;[1 1 1] Update the display score gradually
  (`KismetSystemLibrary.K2_SetTimerDelegate` (delegate `Smooth Update`) 0.011111 true))

(event `Smooth Update`
  (bind _score_shift_speed (`self.Score Shift Speed`))
  (bind _center_shift_speed (`self.Center Shift Speed`))
  (bind _score_shift_speed_2 (`self.Score Shift Speed`))
  (bind _returnvalue (- (`self.Center Offset`) (`self.Center Display Offset`)))
  (bind _returnvalue_2 (- (`self.Get Score` (`self.Player1`)) (`self.Player1 Display Score`)))
  (bind _returnvalue_3 (- (`self.Get Score` (`self.Player2`)) (`self.Player2 Display Score`)))
  ;[1 1 1] Update the display score gradually
  (`|ExecutionSequence`
    (:`then_0`
      (if (!= 0.0 _returnvalue_2)
        (set `self.Player1 Display Score` (+ (`KismetMathLibrary.FMax` (`KismetMathLibrary.FMin` _returnvalue_2 _score_shift_speed) (* _score_shift_speed -1.0)) (`self.Player1 Display Score`)))))
    (:`then_1`
      (if (!= 0.0 _returnvalue_3)
        (set `self.Player2 Display Score` (+ (`KismetMathLibrary.FMax` (`KismetMathLibrary.FMin` _returnvalue_3 _score_shift_speed_2) (* _score_shift_speed_2 -1.0)) (`self.Player2 Display Score`)))))
    (:`then_2`
      (if (!= 0.0 _returnvalue)
        (bind _output_get (set `self.Center Display Offset` (+ (`KismetMathLibrary.FMax` (`KismetMathLibrary.FMin` _returnvalue _center_shift_speed) (* _center_shift_speed -1.0)) (`self.Center Display Offset`))))
        (`MaterialInstanceDynamic.SetScalarParameterValue` (`self.Thermometer Material`) "Center Offset" _output_get)
        (`self.Light PositionUpdate`)))))

(fn `Get Score`
  (params (Player :type "/Game/Blueprint/Pawns/BasePlayer_Blueprint Object Reference"))
  (returns (Score :type "Float (double-precision)"))
  (`/Engine/EditorBlueprintResources/StandardMacros.IsValid` Player
    (:`Is Valid`
      (return (`/Game/Blueprint/Pawns/BasePlayer_Blueprint.Score` Player)))
    (:`Is Not Valid`
      (return 0.0))))

(fn `GetPlayerZonePercentage`
  (returns (Percentage :type "Float (double-precision)"))
  (return (/ (`self.Player Zone Size`) (/ (.y (`SceneComponent.K2_GetComponentScale` (`self.Floor`))) (.x (`SceneComponent.K2_GetComponentScale` (`self.Floor`)))))))

(fn `GetThermometerLowerLocation`
  (returns (Location :type "Float (double-precision)"))
  (return (* (- 1.0 (`self.GetPlayerZonePercentage`)) (* 50 (.y (`SceneComponent.K2_GetComponentScale` (`self.Floor`)))))))

(fn `GetThermometerTopLocation`
  (returns (Location :type "Float (double-precision)"))
  (return (* (`self.GetThermometerLowerLocation`) (`self.Center Offset`))))

(fn `Has Required Score To Open Light`
  (params (`Required Offset` :type "Float (double-precision)") (`Is Player1` :type Boolean))
  (returns (`Required Score` :type Boolean))
  (if `Is Player1`
    (return (>= (/ 0.0 (- (`self.Get Score` (`self.Player1`)) (`self.Center Offset`))) `Required Offset`))
    (else
      (return (>= (/ 0.0 (+ (`self.Get Score` (`self.Player2`)) (`self.Center Offset`))) `Required Offset`)))))

(fn `Place Light`
  (params (`Light Offset` :type "Float (double-precision)") (`Is Player 1` :type Boolean) (`Light Mesh` :type "StaticMeshComponent Object Reference"))
  (`SceneComponent.K2_SetWorldLocation` `Light Mesh` (`KismetMathLibrary.MakeVector` 0.0 (+ (* (`self.GetThermometerTopLocation`) `Light Offset`) (* (`self.GetThermometerLowerLocation`) (- 1.0 `Light Offset`) (`KismetMathLibrary.Conv_IntToDouble` (- (* (`KismetMathLibrary.Conv_BoolToInt` `Is Player 1`) 2) 1)))) -1.0) false false))

(fn `UserConstructionScript`)