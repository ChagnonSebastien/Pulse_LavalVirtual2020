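; Floor thermometer actor that displays two player scores through a dynamic material instance on its Plane.
; Two timelines supply a HeartBeat curve, scaled by BeatRange and added to each score, to drive the Player1 and Player2 material parameters as a pulse.
; Numpad development shortcuts adjust both scores, the material Offset and Player 1's pulse rate.
; The graph never explicitly starts either timeline.
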(event `self.ReceiveBeginPlay`
  ;[1 1 1] Initialization
  (bind _returnvalue (`PrimitiveComponent.CreateDynamicMaterialInstance` (`self.Plane`) 0 "/Game/Assets/Thermometer/Thermometer_Material_v1.Thermometer_Material_v1" "None"))
  (set `self.Material` _returnvalue)
  ;[1 1 1] Key shortcuts for development purposes
  (`self.EnableInput` (`GameplayStatics.GetPlayerController` 0)))

(event `Key|NumPadSeven`
  (params (Key :type "Key Structure"))
  ;[1 1 1] Key shortcuts for development purposes
  (:`Pressed`
    (set `self.Player1 Score` (+ (`self.Player1 Score`) 0.05))))

(event `Key|NumPadOne`
  (params (Key :type "Key Structure"))
  ;[1 1 1] Key shortcuts for development purposes
  (:`Pressed`
    (set `self.Player1 Score` (- (`self.Player1 Score`) 0.05))))

(event `Key|NumPadNine`
  (params (Key :type "Key Structure"))
  ;[1 1 1] Key shortcuts for development purposes
  (:`Pressed`
    (set `self.Player2 Score` (+ (`self.Player2 Score`) 0.05))))

(event `Key|NumPadThree`
  (params (Key :type "Key Structure"))
  ;[1 1 1] Key shortcuts for development purposes
  (:`Pressed`
    (set `self.Player2 Score` (- (`self.Player2 Score`) 0.05))))

(event `Key|NumPadFour`
  (params (Key :type "Key Structure"))
  ;[1 1 1] Key shortcuts for development purposes
  (:`Pressed`
    (set `self.Offset` (+ (`self.Offset`) 0.05))
    (`MaterialInstanceDynamic.SetScalarParameterValue` (`self.Material`) "Offset" (`self.Offset`) :!label _label)))

(event `Key|NumPadSix`
  (params (Key :type "Key Structure"))
  ;[1 1 1] Key shortcuts for development purposes
  (:`Pressed`
    (set `self.Offset` (- (`self.Offset`) 0.05))
    (goto _label)))

(event `Key|NumPadEight`
  (params (Key :type "Key Structure"))
  (bind _timeline_player1 (`self.Timeline Player1`))
  ;[1 1 1] Key shortcuts for development purposes
  (:`Pressed`
    (`TimelineComponent.SetPlayRate` _timeline_player1 (+ (`TimelineComponent.GetPlayRate` _timeline_player1) 0.016667))))

(event `Key|NumPadTwo`
  (params (Key :type "Key Structure"))
  (bind _timeline_player1 (`self.Timeline Player1`))
  ;[1 1 1] Key shortcuts for development purposes
  (:`Pressed`
    (`TimelineComponent.SetPlayRate` _timeline_player1 (- (`TimelineComponent.GetPlayRate` _timeline_player1) 0.016667))))

(fn `UserConstructionScript`)