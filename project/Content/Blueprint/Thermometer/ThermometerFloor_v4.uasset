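; Two-player thermometer floor that displays each player's multiplier and heart rate through dynamic materials on the floor, player bases and side markers.
; A looping timer eases display multipliers toward GameState values, revealing and coloring side markers as thresholds are reached.
; Heart-rate events set the play rate of per-player timelines meant to pulse the bases and score fill.
; Room-scale events re-lay out bases, markers and GameState player positions from the floor's scale.
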(event `self.ReceiveBeginPlay`
  ;[1 1 1] Initialization
  (`|ExecutionSequence`
    (:`then_0`
      (bind _returnvalue (`PrimitiveComponent.CreateDynamicMaterialInstance` (`self.Floor`) 0 "/Game/Assets/Thermometer/Thermometer_Material_v4.Thermometer_Material_v4" "None"))
      (bind _output_get (set `self.Thermometer Material` _returnvalue))
      (`MaterialInstanceDynamic.SetVectorParameterValue` _output_get "Player1 Color" (`KismetMathLibrary.Conv_ColorToLinearColor` (`self.Player 1 Color`)))
      (`MaterialInstanceDynamic.SetVectorParameterValue` _output_get "Player2 Color" (`KismetMathLibrary.Conv_ColorToLinearColor` (`self.Player 2 Color`)))
      (`MaterialInstanceDynamic.SetVectorParameterValue` _output_get "Base Color" (`KismetMathLibrary.Conv_ColorToLinearColor` (`self.Base Color`)))
      (`MaterialInstanceDynamic.SetScalarParameterValue` _output_get "Player Zone Percentage" (`self.GetPlayerZonePercentage`)))
    (:`then_1`
      (bind _returnvalue_2 (`PrimitiveComponent.CreateDynamicMaterialInstance` (`self.Player1 Base`) 0 "/Game/Assets/Thermometer/ThermometerEnd_Material_v4.ThermometerEnd_Material_v4" "None"))
      (`KismetArrayLibrary.Array_Set` (`self.Base Materials`) 0 _returnvalue_2 true)
      (`MaterialInstanceDynamic.SetVectorParameterValue` _returnvalue_2 "Player Color" (`KismetMathLibrary.Conv_ColorToLinearColor` (`self.Player 1 Color`)))
      (`MaterialInstanceDynamic.SetVectorParameterValue` _returnvalue_2 "Base Color" (`KismetMathLibrary.Conv_ColorToLinearColor` (`self.Base Color`))))
    (:`then_2`
      (bind _returnvalue_3 (`PrimitiveComponent.CreateDynamicMaterialInstance` (`self.Player2 Base`) 0 "/Game/Assets/Thermometer/ThermometerEnd_Material_v4.ThermometerEnd_Material_v4" "None"))
      (`KismetArrayLibrary.Array_Set` (`self.Base Materials`) 1 _returnvalue_3 true)
      (`MaterialInstanceDynamic.SetVectorParameterValue` _returnvalue_3 "Player Color" (`KismetMathLibrary.Conv_ColorToLinearColor` (`self.Player 2 Color`)))
      (`MaterialInstanceDynamic.SetVectorParameterValue` _returnvalue_3 "Base Color" (`KismetMathLibrary.Conv_ColorToLinearColor` (`self.Base Color`))))
    (:`then_3`
      (`self.Colour Side Lights`)
      (`self.Start Smooth Score Update`)
      (bind _asmain_game_state (cast `/Game/Main_GameState` (`GameplayStatics.GetGameState`)))
      (bind _output_get_2 (set `self.Game State Reference` _asmain_game_state))
      (add `/Game/Main_GameState.HeartRate Updated` _output_get_2 (delegate `Update HeartRate`))
      (`TimelineComponent.SetPlayRate` (`self.Timeline Player1`) 0.0)
      (`TimelineComponent.SetPlayRate` (`self.Timeline Player2`) 0.0)
      (add `/Game/Main_GameState.Room Scaled` _output_get_2 (delegate `Rescale Floor Material`))
      (add `/Game/Main_GameState.Scene Reset` _output_get_2 (delegate `HandleSceneReset`)))))

(event `HandleSceneReset`
  (`SceneComponent.SetVisibility` (`self.Multiplayers`) false true))

(event `Colour Side Lights`
  ;[1 1 1] Sets the colors of each of the side lights
  (`|ExecutionSequence`
    (:`then_0`
      (for _array_element (`SceneComponent.GetChildrenComponents` (`self.Player1 Multipliers`) false)
        (bind _asstatic_mesh_component (cast `StaticMeshComponent` _array_element))
        (bind _returnvalue (`PrimitiveComponent.CreateDynamicMaterialInstance` _asstatic_mesh_component 0 "/Game/Assets/Multipliers/Multiplier_Material.Multiplier_Material" "None"))
        (bind _returnvalue_2 (`KismetArrayLibrary.Array_Add` (`self.Player1 Multiplier Materials`) _returnvalue))
        (`MaterialInstanceDynamic.SetScalarParameterValue` _returnvalue "Value" (`KismetMathLibrary.Conv_IntToDouble` (+ _returnvalue_2 2)))))
    (:`then_1`
      (for _array_element_2 (`SceneComponent.GetChildrenComponents` (`self.Player2 Multipliers`) false)
        (bind _asstatic_mesh_component_2 (cast `StaticMeshComponent` _array_element_2))
        (bind _returnvalue_3 (`PrimitiveComponent.CreateDynamicMaterialInstance` _asstatic_mesh_component_2 0 "/Game/Assets/Multipliers/Multiplier_Material.Multiplier_Material" "None"))
        (bind _returnvalue_4 (`KismetArrayLibrary.Array_Add` (`self.Player2 Multiplier Materials`) _returnvalue_3))
        (`MaterialInstanceDynamic.SetScalarParameterValue` _returnvalue_3 "Value" (`KismetMathLibrary.Conv_IntToDouble` (+ _returnvalue_4 2)))))))

(event `Update HeartRate`
  (params (`Player ID` :type Integer) (HeartRate :type Integer))
  (bind _returnvalue (/ (`KismetMathLibrary.Conv_IntToDouble` HeartRate) 60.0))
  ;[1 1 1] Update Visual Heart Rate Pulse Speed
  (`MaterialInstanceDynamic.SetScalarParameterValue` (`|GetArrayItem` (`self.Base Materials`) `Player ID`) "HB Visibility" 1.0)
  (switch `int` `Player ID`
    (:`0`
      (`TimelineComponent.SetPlayRate` (`self.Timeline Player1`) _returnvalue))
    (:`1`
      (`TimelineComponent.SetPlayRate` (`self.Timeline Player2`) _returnvalue))))

(event `Rescale Floor Material`
  (bind _percentage (`self.GetPlayerZonePercentage`))
  (bind _player2_base (`self.Player2 Base`))
  (bind _player1_base (`self.Player1 Base`))
  (bind _x (.x (`SceneComponent.K2_GetComponentScale` (`self.Floor`))))
  (bind _returnvalue (* (`KismetMathLibrary.MakeVector` _x _x _x) 0.75))
  (bind _returnvalue_2 (* (- 1.0 (/ _percentage 2.0)) (* 50 (.y (`SceneComponent.K2_GetComponentScale` (`self.Floor`))))))
  (bind _returnvalue_3 (`KismetMathLibrary.MakeVector` 0.0 _returnvalue_2 0.1))
  (bind _returnvalue_4 (`KismetMathLibrary.MakeVector` 0.0 (* _returnvalue_2 -1.0) 0.1))
  ;[1 1 1] Startup sequence
  (`self.Light PositionUpdate`)
  (`MaterialInstanceDynamic.SetScalarParameterValue` (`self.Thermometer Material`) "Player Zone Percentage" _percentage)
  (`SceneComponent.SetWorldScale3D` _player1_base _returnvalue)
  (`SceneComponent.K2_SetWorldLocation` _player1_base _returnvalue_3 false false)
  (`/Game/Main_GameState.Update Player Position` (`self.Game State Reference`) 0 (+ _returnvalue_3 (0.0 0.0 0.0)))
  (`SceneComponent.SetWorldScale3D` _player2_base _returnvalue)
  (`SceneComponent.K2_SetWorldLocation` _player2_base _returnvalue_4 false false)
  (`/Game/Main_GameState.Update Player Position` (`self.Game State Reference`) 1 (+ _returnvalue_4 (0.0 0.0 0.0)))
  (`|ExecutionSequence`
    (:`then_0`
      (for _array_element (`SceneComponent.GetChildrenComponents` (`self.Player1 Multipliers`) false)
        (bind _x_2 (.x (`SceneComponent.K2_GetComponentScale` _array_element)))
        (`SceneComponent.SetWorldScale3D` _array_element (`KismetMathLibrary.MakeVector` _x_2 _x_2 (.z (`SceneComponent.K2_GetComponentScale` _array_element))))))
    (:`then_1`
      (for _array_element_2 (`SceneComponent.GetChildrenComponents` (`self.Player2 Multipliers`) false)
        (bind _x_3 (.x (`SceneComponent.K2_GetComponentScale` _array_element_2)))
        (`SceneComponent.SetWorldScale3D` _array_element_2 (`KismetMathLibrary.MakeVector` _x_3 _x_3 (.z (`SceneComponent.K2_GetComponentScale` _array_element_2))))))))

(event `Lightup Side Indicators`
  (bind _multipliers_offsets (`self.Multipliers Offsets`))
  ;[1 1 1] Startup sequence
  (`|ExecutionSequence`
    (:`then_0`
      (for (_array_element _array_index) _multipliers_offsets
        (bind _returnvalue (`SceneComponent.GetChildComponent` (`self.Player1 Multipliers`) _array_index))
        (if (and (<= _array_element (`self.Player1 Display Multiplier`)) (not (`SceneComponent.IsVisible` _returnvalue)))
          (`SceneComponent.SetVisibility` _returnvalue true true))
        (`self.Check Light Status` true)))
    (:`then_1`
      (for (_array_element_2 _array_index_2) _multipliers_offsets
        (bind _returnvalue_2 (`SceneComponent.GetChildComponent` (`self.Player2 Multipliers`) _array_index_2))
        (if (and (<= _array_element_2 (`self.Player2 Display Multiplier`)) (not (`SceneComponent.IsVisible` _returnvalue_2)))
          (`SceneComponent.SetVisibility` _returnvalue_2 true true))
        (`self.Check Light Status` false)))))

(event `Light PositionUpdate`
  ;[1 1 1] Updates the location of the side indicators
  (`|ExecutionSequence`
    (:`then_0`
      (for (_array_element _array_index) (`SceneComponent.GetChildrenComponents` (`self.Player1 Multipliers`) false)
        (bind _asstatic_mesh_component (cast `StaticMeshComponent` _array_element))
        (`self.Place Light` (`|GetArrayItem` (`self.Multipliers Offsets`) _array_index) true _asstatic_mesh_component)))
    (:`then_1`
      (for (_array_element_2 _array_index_2) (`SceneComponent.GetChildrenComponents` (`self.Player2 Multipliers`) false)
        (bind _asstatic_mesh_component_2 (cast `StaticMeshComponent` _array_element_2))
        (`self.Place Light` (`|GetArrayItem` (`self.Multipliers Offsets`) _array_index_2) false _asstatic_mesh_component_2)))))

(event `Close Side Lights`
  ;[1 1 1] Startup sequence
  (`SceneComponent.SetVisibility` (`self.Player1 Multipliers`) false true)
  (`SceneComponent.SetVisibility` (`self.Player2 Multipliers`) false true))

(event `Check Light Status`
  (params (`Is Player1` :type Boolean))
  ;[1 1 1] Side Light Controller
  (if `Is Player1`
    (for (_ _array_index) (`SceneComponent.GetChildrenComponents` (`self.Player1 Multipliers`) false)
      (bind _required_score (`self.Has Required Score To Open Light` (`|GetArrayItem` (`self.Multipliers Offsets`) _array_index) true))
      (`MaterialInstanceDynamic.SetVectorParameterValue` (`|GetArrayItem` (`self.Player1 Multiplier Materials`) _array_index) "Color" (`KismetMathLibrary.SelectColor` (struct :`R` 0.85 :`G` 0.15 :`A` 1.0) (struct :`R` 0.1 :`G` 0.1 :`B` 0.1 :`A` 1.0) _required_score)))
    (else
      (for (_ _array_index_2) (`SceneComponent.GetChildrenComponents` (`self.Player2 Multipliers`) false)
        (bind _required_score_2 (`self.Has Required Score To Open Light` (`|GetArrayItem` (`self.Multipliers Offsets`) _array_index_2)))
        (`MaterialInstanceDynamic.SetVectorParameterValue` (`|GetArrayItem` (`self.Player2 Multiplier Materials`) _array_index_2) "Color" (`KismetMathLibrary.SelectColor` (struct :`G` 0.15 :`B` 0.85 :`A` 1.0) (struct :`R` 0.1 :`G` 0.1 :`B` 0.1 :`A` 1.0) _required_score_2))))))

(event `Start Smooth Score Update`
  ;[1 1 1] Update the display score gradually
  (`KismetSystemLibrary.K2_SetTimerDelegate` (delegate `Smooth Update`) 0.011111 true))

(event `Smooth Update`
  (bind _score_shift_speed (`self.Score Shift Speed`))
  (bind _score_shift_speed_2 (`self.Score Shift Speed`))
  (bind _returnvalue (- (`KismetMathLibrary.Conv_IntToDouble` (`/Game/Main_GameState.Get Multiplier` (`self.Game State Reference`) 0)) (`self.Player1 Display Multiplier`)))
  (bind _returnvalue_2 (- (`KismetMathLibrary.Conv_IntToDouble` (`/Game/Main_GameState.Get Multiplier` (`self.Game State Reference`) 1)) (`self.Player2 Display Multiplier`)))
  ;[1 1 1] Update the display score gradually
  (`|ExecutionSequence`
    (:`then_0`
      (if (!= 0.0 _returnvalue)
        (set `self.Player1 Display Multiplier` (+ (`KismetMathLibrary.FMax` (`KismetMathLibrary.FMin` _returnvalue _score_shift_speed) (* _score_shift_speed -1.0)) (`self.Player1 Display Multiplier`)))))
    (:`then_1`
      (if (!= 0.0 _returnvalue_2)
        (set `self.Player2 Display Multiplier` (+ (`KismetMathLibrary.FMax` (`KismetMathLibrary.FMin` _returnvalue_2 _score_shift_speed_2) (* _score_shift_speed_2 -1.0)) (`self.Player2 Display Multiplier`)))))
    (:`then_2`
      (`self.Lightup Side Indicators`))))

(fn `GetPlayerZonePercentage`
  (returns (Percentage :type "Float (double-precision)"))
  (return (/ (`self.Player Zone Size`) (/ (.y (`SceneComponent.K2_GetComponentScale` (`self.Floor`))) (.x (`SceneComponent.K2_GetComponentScale` (`self.Floor`)))))))

(fn `GetThermometerLowerLocation`
  (returns (Location :type "Float (double-precision)"))
  (return (* (- 1.0 (`self.GetPlayerZonePercentage`)) (* 50 (.y (`SceneComponent.K2_GetComponentScale` (`self.Floor`)))))))

(fn `GetThermometerTopLocation`
  (returns (Location :type "Float (double-precision)"))
  (return (* (`self.GetThermometerLowerLocation`) (`self.Center Display Offset`))))

(fn `Has Required Score To Open Light`
  (params (`Required Offset` :type "Float (double-precision)") (`Is Player1` :type Boolean))
  (returns (`Required Score` :type Boolean))
  (if `Is Player1`
    (return (>= (/ (`self.Player1 Display Multiplier`) (- 1.0 (`self.Center Offset`))) `Required Offset`))
    (else
      (return (>= (/ (`self.Player2 Display Multiplier`) (+ 1.0 (`self.Center Offset`))) `Required Offset`)))))

(fn `Place Light`
  (params (`Light Offset` :type "Float (double-precision)") (`Is Player 1` :type Boolean) (`Light Mesh` :type "StaticMeshComponent Object Reference"))
  (bind _returnvalue (/ `Light Offset` 6.0))
  (`SceneComponent.K2_SetWorldLocation` `Light Mesh` (`KismetMathLibrary.MakeVector` (.x (`SceneComponent.K2_GetComponentLocation` `Light Mesh`)) (+ (* (`self.GetThermometerTopLocation`) _returnvalue) (* (`self.GetThermometerLowerLocation`) (- 1.0 _returnvalue) (`KismetMathLibrary.Conv_IntToDouble` (- (* (`KismetMathLibrary.Conv_BoolToInt` `Is Player 1`) 2) 1))))) false false))

(fn `UserConstructionScript`)