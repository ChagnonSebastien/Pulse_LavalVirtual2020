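; A hand-held racket Blueprint that shifts its Racket component sideways according to which hand it belongs to.
; The construction script switches on Side and applies a small, mirrored world Y offset for right or left.
; The Hit event is empty.
; Disconnected logic would cast the other actor to Ball_Blueprint and play force feedback scaled by the ball's speed, but it never runs.
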(event `self.ReceiveHit`
  (params (MyComp :type "PrimitiveComponent Object Reference") (Other :type "Actor Object Reference") (OtherComp :type "PrimitiveComponent Object Reference") (bSelfMoved :type Boolean) (HitLocation :type "Vector Structure") (HitNormal :type "Vector Structure") (NormalImpulse :type "Vector Structure") (Hit :type "HitResult Structure (by ref)")))

(fn `UserConstructionScript`
  (bind _racket (`self.Racket`))
  (switch `string` (`self.Side`)
    (:`Right`
      (`SceneComponent.K2_AddWorldOffset` _racket (0.0 5.0 0.0) false false))
    (:`Left`
      (`SceneComponent.K2_AddWorldOffset` _racket (0.0 -5.0 0.0) false false))))