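; Thermometer-style floor showing two players' scores through a dynamic material, with green, yellow and red side lights per player.
; An offset shifts the shared top point, repositioning the lights, which illuminate when each score, scaled by offset, passes their thresholds.
; Numpad development keys adjust scores, offset and Player 1's timeline play rate.
; Heartbeat timelines would feed scores and pulse into the material, but nothing here starts them.
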(event `self.ReceiveBeginPlay`
  ;[1 1 1] Initialization
  (bind _returnvalue (`PrimitiveComponent.CreateDynamicMaterialInstance` (`self.Floor`) 0 "/Game/Assets/Thermometer/Thermometer_Material_v2.Thermometer_Material_v2" "None"))
  (bind _output_get (set `self.Material` _returnvalue))
  (`MaterialInstanceDynamic.SetScalarParameterValue` _output_get "Player Zone Percentage" (`self.Player Zone Percentage`))
  (`self.Enable Keyboard`)
  (`self.Colour Side Lights`)
  (set `self.FloorScaleY` (.y (`SceneComponent.K2_GetComponentScale` (`self.Floor`))))
  (`self.Light Position Update`))

(event `Key|NumPadSeven`
  (params (Key :type "Key Structure"))
  ;[1 1 1] Key shortcuts for development purposes
  (:`Pressed`
    (set `self.Player2 Score` (+ (`self.Player2 Score`) 0.05))
    (`self.Check Side Light Status` :!label _label)))

(event `Enable Keyboard`
  ;[1 1 1] Key shortcuts for development purposes
  (`self.EnableInput` (`GameplayStatics.GetPlayerController` 0)))

(event `Key|NumPadOne`
  (params (Key :type "Key Structure"))
  ;[1 1 1] Key shortcuts for development purposes
  (:`Pressed`
    (set `self.Player2 Score` (- (`self.Player2 Score`) 0.05))
    (goto _label)))

(event `Key|NumPadNine`
  (params (Key :type "Key Structure"))
  ;[1 1 1] Key shortcuts for development purposes
  (:`Pressed`
    (set `self.Player1 Score` (+ (`self.Player1 Score`) 0.05))
    (goto _label)))

(event `Key|NumPadThree`
  (params (Key :type "Key Structure"))
  ;[1 1 1] Key shortcuts for development purposes
  (:`Pressed`
    (set `self.Player1 Score` (- (`self.Player1 Score`) 0.05))
    (goto _label)))

(event `Colour Side Lights`
  ;[1 1 1] Sets the colors of each of the side lights
  (`|ExecutionSequence`
    (:`then_0`
      (bind _returnvalue (`PrimitiveComponent.CreateDynamicMaterialInstance` (`self.P1_side_green`) 0 "/Game/Assets/Thermometer/side_light_material.side_light_material" "None"))
      (bind _output_get (set `self.P1 Side Green Material` _returnvalue))
      (`MaterialInstanceDynamic.SetScalarParameterValue` _output_get "Green" 1.0))
    (:`then_1`
      (bind _returnvalue_2 (`PrimitiveComponent.CreateDynamicMaterialInstance` (`self.P1_side_yellow`) 0 "/Game/Assets/Thermometer/side_light_material.side_light_material" "None"))
      (bind _output_get_2 (set `self.P1 Side Yellow Material` _returnvalue_2))
      (`MaterialInstanceDynamic.SetScalarParameterValue` _output_get_2 "Green" 1.0)
      (`MaterialInstanceDynamic.SetScalarParameterValue` _output_get_2 "Red" 1.0))
    (:`then_2`
      (bind _returnvalue_3 (`PrimitiveComponent.CreateDynamicMaterialInstance` (`self.P1_side_red`) 0 "/Game/Assets/Thermometer/side_light_material.side_light_material" "None"))
      (bind _output_get_3 (set `self.P1 Side Red Material` _returnvalue_3))
      (`MaterialInstanceDynamic.SetScalarParameterValue` _output_get_3 "Red" 1.0))
    (:`then_3`
      (bind _returnvalue_4 (`PrimitiveComponent.CreateDynamicMaterialInstance` (`self.P2_side_green`) 0 "/Game/Assets/Thermometer/side_light_material.side_light_material" "None"))
      (bind _output_get_4 (set `self.P2 Side Green Material` _returnvalue_4))
      (`MaterialInstanceDynamic.SetScalarParameterValue` _output_get_4 "Green" 1.0))
    (:`then_4`
      (bind _returnvalue_5 (`PrimitiveComponent.CreateDynamicMaterialInstance` (`self.P2_side_yellow`) 0 "/Game/Assets/Thermometer/side_light_material.side_light_material" "None"))
      (bind _output_get_5 (set `self.P2 Side Yellow Material` _returnvalue_5))
      (`MaterialInstanceDynamic.SetScalarParameterValue` _output_get_5 "Green" 1.0)
      (`MaterialInstanceDynamic.SetScalarParameterValue` _output_get_5 "Red" 1.0))
    (:`then_5`
      (bind _returnvalue_6 (`PrimitiveComponent.CreateDynamicMaterialInstance` (`self.P2_side_red`) 0 "/Game/Assets/Thermometer/side_light_material.side_light_material" "None"))
      (bind _output_get_6 (set `self.P2 Side Red Material` _returnvalue_6))
      (`MaterialInstanceDynamic.SetScalarParameterValue` _output_get_6 "Red" 1.0))))

(event `Key|NumPadSix`
  (params (Key :type "Key Structure"))
  ;[1 1 1] Key shortcuts for development purposes
  (:`Pressed`
    (set `self.Offset` (+ (`self.Offset`) 0.05))
    (`MaterialInstanceDynamic.SetScalarParameterValue` (`self.Material`) "Offset" (`self.Offset`) :!label _label_2)
    (`self.Light Position Update`)))

(event `Key|NumPadFour`
  (params (Key :type "Key Structure"))
  ;[1 1 1] Key shortcuts for development purposes
  (:`Pressed`
    (set `self.Offset` (- (`self.Offset`) 0.05))
    (goto _label_2)))

(event `Key|NumPadEight`
  (params (Key :type "Key Structure"))
  (bind _timeline_player1 (`self.Timeline Player1`))
  ;[1 1 1] Key shortcuts for development purposes
  (:`Pressed`
    (`TimelineComponent.SetPlayRate` _timeline_player1 (+ (`TimelineComponent.GetPlayRate` _timeline_player1) 0.016667))))

(event `Key|NumPadTwo`
  (params (Key :type "Key Structure"))
  (bind _timeline_player1 (`self.Timeline Player1`))
  ;[1 1 1] Key shortcuts for development purposes
  (:`Pressed`
    (`TimelineComponent.SetPlayRate` _timeline_player1 (- (`TimelineComponent.GetPlayRate` _timeline_player1) 0.016667))))

(event `Light Position Update`
  (bind _red_light_offset (`self.Red Light Offset`))
  (bind _green_light_offset (`self.Green Light Offset`))
  (bind _yellow_light_offset (`self.Yellow Light Offset`))
  (bind _green_light_offset_2 (`self.Green Light Offset`))
  (bind _yellow_light_offset_2 (`self.Yellow Light Offset`))
  (bind _red_light_offset_2 (`self.Red Light Offset`))
  ;[1 1 1] Updates the location of the side indicators
  (`|ExecutionSequence`
    (:`then_0`
      (bind _location (`self.GetThermometerTopLocation`))
      (bind _location_2 (`self.GetThermometerLowerLocation`))
      (`SceneComponent.K2_SetRelativeLocation` (`self.P1_side_green`) (`KismetMathLibrary.MakeVector` 0.0 (+ (* _location _green_light_offset_2) (* _location_2 (- 1.0 _green_light_offset_2)))) false false))
    (:`then_1`
      (bind _location_3 (`self.GetThermometerTopLocation`))
      (bind _location_4 (`self.GetThermometerLowerLocation`))
      (`SceneComponent.K2_SetRelativeLocation` (`self.P1_side_yellow`) (`KismetMathLibrary.MakeVector` 0.0 (+ (* _location_3 _yellow_light_offset_2) (* _location_4 (- 1.0 _yellow_light_offset_2)))) false false))
    (:`then_2`
      (bind _location_5 (`self.GetThermometerTopLocation`))
      (bind _location_6 (`self.GetThermometerLowerLocation`))
      (`SceneComponent.K2_SetRelativeLocation` (`self.P1_side_red`) (`KismetMathLibrary.MakeVector` 0.0 (+ (* _location_5 _red_light_offset_2) (* _location_6 (- 1.0 _red_light_offset_2)))) false false))
    (:`then_3`
      (bind _location_7 (`self.GetThermometerTopLocation`))
      (bind _location_8 (`self.GetThermometerLowerLocation`))
      (`SceneComponent.K2_SetRelativeLocation` (`self.P2_side_green`) (`KismetMathLibrary.MakeVector` 0.0 (+ (* _location_7 _green_light_offset) (* (* _location_8 -1.0) (- 1.0 _green_light_offset)))) false false))
    (:`then_4`
      (bind _location_9 (`self.GetThermometerTopLocation`))
      (bind _location_10 (`self.GetThermometerLowerLocation`))
      (`SceneComponent.K2_SetRelativeLocation` (`self.P2_side_yellow`) (`KismetMathLibrary.MakeVector` 0.0 (+ (* _location_9 _yellow_light_offset) (* (* _location_10 -1.0) (- 1.0 _yellow_light_offset)))) false false))
    (:`then_5`
      (bind _location_11 (`self.GetThermometerTopLocation`))
      (bind _location_12 (`self.GetThermometerLowerLocation`))
      (`SceneComponent.K2_SetRelativeLocation` (`self.P2_side_red`) (`KismetMathLibrary.MakeVector` 0.0 (+ (* _location_11 _red_light_offset) (* (* _location_12 -1.0) (- 1.0 _red_light_offset)))) false false))
    (:`then_6`
      (`self.Check Side Light Status`))))

(event `Check Side Light Status`
  (bind _returnvalue (/ (`self.Player1 Score`) (- 1.0 (`self.Offset`))))
  (bind _returnvalue_2 (/ (`self.Player2 Score`) (+ 1.0 (`self.Offset`))))
  ;[1 1 1] Light the side lights if the player score is high enough
  (`|ExecutionSequence`
    (:`then_0`
      (`MaterialInstanceDynamic.SetScalarParameterValue` (`self.P1 Side Green Material`) "Intensity" (`KismetMathLibrary.Conv_BoolToDouble` (>= _returnvalue (`self.Green Light Offset`)))))
    (:`then_1`
      (`MaterialInstanceDynamic.SetScalarParameterValue` (`self.P1 Side Yellow Material`) "Intensity" (`KismetMathLibrary.Conv_BoolToDouble` (>= _returnvalue (`self.Yellow Light Offset`)))))
    (:`then_2`
      (`MaterialInstanceDynamic.SetScalarParameterValue` (`self.P1 Side Red Material`) "Intensity" (`KismetMathLibrary.Conv_BoolToDouble` (>= _returnvalue (`self.Red Light Offset`)))))
    (:`then_3`
      (`MaterialInstanceDynamic.SetScalarParameterValue` (`self.P2 Side Green Material`) "Intensity" (`KismetMathLibrary.Conv_BoolToDouble` (>= _returnvalue_2 (`self.Green Light Offset`)))))
    (:`then_4`
      (`MaterialInstanceDynamic.SetScalarParameterValue` (`self.P2 Side Yellow Material`) "Intensity" (`KismetMathLibrary.Conv_BoolToDouble` (>= _returnvalue_2 (`self.Yellow Light Offset`)))))
    (:`then_5`
      (`MaterialInstanceDynamic.SetScalarParameterValue` (`self.P2 Side Red Material`) "Intensity" (`KismetMathLibrary.Conv_BoolToDouble` (>= _returnvalue_2 (`self.Red Light Offset`)))))))

(fn `GetThermometerLowerLocation`
  (returns (Location :type "Float (double-precision)"))
  (return (* (* 50 (`self.FloorScaleY`)) (- 1.0 (`self.Player Zone Percentage`)))))

(fn `GetThermometerTopLocation`
  (returns (Location :type "Float (double-precision)"))
  (bind _location (`self.GetThermometerLowerLocation`))
  (return (* _location (`self.Offset`))))

(fn `UserConstructionScript`)