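; Hand racket Blueprint that triggers glove haptics when its Racket component hits something.
; On a hit, it casts its parent actor to the base player Blueprint and continues only if that player has ownership.
; The Side value selects the left or right glove to vibrate and prints a debug letter.
; A side-based racket offset exists in the construction script graph but is unconnected and never runs.
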(event `self.Racket.OnComponentHit`
  (params (HitComponent :type "PrimitiveComponent Object Reference") (OtherActor :type "Actor Object Reference") (OtherComp :type "PrimitiveComponent Object Reference") (NormalImpulse :type "Vector Structure") (Hit :type "HitResult Structure (by ref)"))
  (bind _asbase_player_blueprint (cast `/Game/Blueprint/Pawns/BasePlayer_Blueprint` (`self.GetParentActor`)))
  (if (`/Game/Blueprint/Pawns/BasePlayer_Blueprint.Has Ownership` _asbase_player_blueprint)
    (switch `string` (`self.Side`)
      (:`Left`
        (`MotionCaptureFunctionLibrary.VibrateLeftGlove` 500)
        (`KismetSystemLibrary.PrintString` "l"))
      (:`Right`
        (`MotionCaptureFunctionLibrary.VibrateRightGlove` 500)
        (`KismetSystemLibrary.PrintString` "r")))))

(fn `UserConstructionScript`)