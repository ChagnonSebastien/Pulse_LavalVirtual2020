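; Lobby pawn that lets the player host or join a LAN multiplayer game through input actions.
; Host creates a ten-connection session and opens MainMap as a listen server.
; Join searches for sessions and joins the first result without checking that the list is non-empty.
; Search and join progress, plus failures, are reported only through on-screen debug prints.
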(event `InputAction|Host`
  (params (Key :type "Key Structure"))
  ;[1 1 1] Host Session
  (:`Pressed`
    (`CreateSessionCallbackProxy.CreateSession` (`GameplayStatics.GetPlayerController` 0) 10 true
      (:`OnSuccess`
        (`GameplayStatics.OpenLevel` "MainMap" true "listen"))
      (:`OnFailure`
        (`KismetSystemLibrary.PrintString` "Failed")))))

(event `InputAction|Join`
  (params (Key :type "Key Structure"))
  ;[1 1 1] Join Session
  (:`Pressed`
    (`KismetSystemLibrary.PrintString` "Searching sessions..." true true (struct :`G` 0.66 :`B` 1.0 :`A` 1.0) 10.0)
    (bind _results (`FindSessionsCallbackProxy.FindSessions` (`GameplayStatics.GetPlayerController` 0) 10 true)
      (:`OnSuccess`
        (bind _output (`|GetArrayItem` _results))
        (`KismetSystemLibrary.PrintString` (`KismetStringLibrary.Concat_StrStr` "Found session: " (`FindSessionsCallbackProxy.GetServerName` _output)) true true (struct :`G` 0.66 :`B` 1.0 :`A` 1.0) 10.0)
        (`JoinSessionCallbackProxy.JoinSession` (`GameplayStatics.GetPlayerController` 0) _output
          (:`OnSuccess`
            (`KismetSystemLibrary.PrintString` "Joined session" true true (struct :`G` 0.66 :`B` 1.0 :`A` 1.0) 10.0))
          (:`OnFailure`
            (`KismetSystemLibrary.PrintString` "Failed to join session" true true (struct :`R` 1.0 :`G` 0.006241 :`A` 1.0) 10.0))))
      (:`OnFailure`
        (`KismetSystemLibrary.PrintString` "Error while trying to find sessions" true true (struct :`R` 1.0 :`B` 0.035091 :`A` 1.0) 10.0)))))

(fn `UserConstructionScript`)