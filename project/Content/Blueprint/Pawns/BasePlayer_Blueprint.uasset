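; Base VR player pawn for a scored match that tracks the player's height and heart rate, with color set by replicated player Id.
; It subscribes to Main_GameState events, spawning and updating a scoreboard and end-game widget for the locally controlled player only.
; A heart-rate child actor feeds HR updates and logs game start/end.
; The pawn keeps the lowest reading as baseline, reset with N for a new player.
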(event `StartGame`
  (bind _z (.z (`SceneComponent.RelativeLocation` (`self.VRCamera`))))
  ;[1 1 1] Set height
  (if (`self.Has Ownership`)
    (if (< _z 100.0)
      (`self.Set height` 170.0)
      (else
        (`self.Set height` _z)))))

(event `self.ReceiveBeginPlay`
  ;[1 1 1] Initialize player position to floor and set height
  (`HeadMountedDisplayFunctionLibrary.SetTrackingOrigin` "Floor")
  (bind _asbase_heart_rate_blueprint (cast `/Game/Blueprint/Biofeedback/BaseHeartRate_Blueprint` (`ChildActorComponent.ChildActor` (`self.HeartRate_Blueprint`))))
  (add `/Game/Blueprint/Biofeedback/BaseHeartRate_Blueprint.HeartRate Updated` _asbase_heart_rate_blueprint (delegate `Update HeartRate`))
  (bind _asmain_game_state (cast `/Game/Main_GameState` (`GameplayStatics.GetGameState`)))
  (set `self.Game State Reference` _asmain_game_state)
  (add `/Game/Main_GameState.Game Started` (`self.Game State Reference`) (delegate `Start Game Event`))
  (add `/Game/Main_GameState.Game Ended` (`self.Game State Reference`) (delegate `Game Ended`))
  (add `/Game/Main_GameState.Score Updated` (`self.Game State Reference`) (delegate `Score Updated`))
  (add `/Game/Main_GameState.Time Updated` (`self.Game State Reference`) (delegate `Add HR Datapoint`))
  (add `/Game/Main_GameState.Scene Reset` (`self.Game State Reference`) (delegate `Scene Reset`))
  (add `/Game/Main_GameState.Time Updated` (`self.Game State Reference`) (delegate `TimeUpdated`)))

(event `TimeUpdated`
  (params (Time :type Integer))
  (if (`self.Has Ownership`)
    (`/Game/Blueprint/Score/Score_Blueprint.Time Updated` (`self.Scoreboard`) Time)))

(event `Update HeartRate`
  (params (HeartRate :type Integer))
  ;[1 1 1] Initialize player position to floor and set height
  (`self.Set HR` HeartRate))

(event `Score Updated`
  (params (`Player ID` :type Integer) (Score :type Integer))
  (if (`self.Has Ownership`)
    (`/Game/Blueprint/EndGame/End_Game_Blueprint.Score Updated` (`self.End game widget`) `Player ID` Score)
    (`/Game/Blueprint/Score/Score_Blueprint.Score Updated` (`self.Scoreboard`) `Player ID` Score)))

(event `Add HR Datapoint`
  (params (Time :type Integer))
  (if (`self.Has Ownership`)
    (`/Game/Blueprint/EndGame/End_Game_Blueprint.Add HR Datapoint` (`self.End game widget`) Time)))

(event `Scene Reset`
  (if (`self.Has Ownership`)
    (`/Game/Blueprint/EndGame/End_Game_Blueprint.Scene Reset` (`self.End game widget`))))

(event `Set HR`
  (params (HR :type Integer))
  (bind _base_hr (`self.Base HR`))
  ;[1 1 1] Replicate heart rate from client to server and from server to client
  (bind _output_get (set `self.hr` HR))
  (`self.HeartRate Updated` (`self.Id`) _output_get)
  (if (or (== _base_hr 0) (> _base_hr HR))
    (set `self.Base HR` _output_get)))

(event `Start Game Event`
  (bind _returnvalue (`KismetMathLibrary.MakeRotator` 0.0 0.0 (+ 90.0 (* 180.0 (`KismetMathLibrary.Conv_IntToDouble` (`self.Id`))))))
  ;[1 1 1] Send Log events to The Wahoo Connector
  (if (`self.Has Ownership`)
    (bind _asbase_heart_rate_blueprint (cast `/Game/Blueprint/Biofeedback/BaseHeartRate_Blueprint` (`ChildActorComponent.ChildActor` (`self.HeartRate_Blueprint`))))
    (`/Game/Blueprint/Biofeedback/BaseHeartRate_Blueprint.Log Game Event` _asbase_heart_rate_blueprint true)
    ;[1 1 1] Add scoreboard
    (bind _returnvalue_2 (`|SpawnActorFromClass` "/Game/Blueprint/Score/Score_Blueprint.Score_Blueprint_C" (`KismetMathLibrary.MakeTransform` (0.0 0.0 350.0) _returnvalue (1.0 0.25 0.25)) "Undefined" "OverrideRootScale" null null))
    (set `self.Scoreboard` _returnvalue_2)
    (bind _returnvalue_3 (`|SpawnActorFromClass` "/Game/Blueprint/EndGame/End_Game_Blueprint.End_Game_Blueprint_C" (`KismetMathLibrary.MakeTransform` (0.0 1.0 200.0) _returnvalue (1.0 0.25 0.25)) "Undefined" "OverrideRootScale" null null))
    (set `self.End game widget` _returnvalue_3)))

(event `Key|N`
  (params (Key :type "Key Structure"))
  ;[1 1 1] Reset the base HR when the player changes with the N  Key
  (:`Pressed`
    (if (`self.Has Ownership`)
      (`self.New Player On Client`))))

(event `New Player On Client`
  ;[1 1 1] Reset the base HR when the player changes with the N  Key
  (set `self.Base HR` 0))

(event `Game Ended`
  (params (`Winner ID` :type Integer))
  ;[1 1 1] Send Log events to The Wahoo Connector
  (if (`self.Has Ownership`)
    (bind _asbase_heart_rate_blueprint (cast `/Game/Blueprint/Biofeedback/BaseHeartRate_Blueprint` (`ChildActorComponent.ChildActor` (`self.HeartRate_Blueprint`))))
    (`/Game/Blueprint/Biofeedback/BaseHeartRate_Blueprint.Log Game Event` _asbase_heart_rate_blueprint false)
    (`/Game/Blueprint/EndGame/End_Game_Blueprint.End Game` (`self.End game widget`) (== `Winner ID` (`self.Id`)))
    ;[1 1 1] Add scoreboard
    (`SceneComponent.SetVisibility` (`/Game/Blueprint/Score/Score_Blueprint.Score_Widget3D` (`self.Scoreboard`)) false true)))

(event `Set height`
  (params (height :type "Float (double-precision)"))
  ;[1 1 1] Replicate height from client to server and from server to client
  (set `self.Height` height))

(event `Set Color`
  (params (Color :type "LinearColor Structure")))

(fn `Has Ownership`
  (returns (isOwner :type Boolean))
  (return (== (`self.GetController`) (`GameplayStatics.GetPlayerController` 0))))

(fn `OnRep_Id`
  (`self.Set Color` (`KismetMathLibrary.SelectColor` (struct :`R` 0.85 :`G` 0.15 :`A` 1.0) (struct :`G` 0.15 :`B` 0.85 :`A` 1.0) (== (`self.Id`) 0))))

(fn `UserConstructionScript`)