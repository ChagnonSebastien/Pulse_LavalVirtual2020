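; Hand component that networks a hand's skeletal mesh transform and finger pose from the owning player to other machines.
; Ownership is the instigator's controller matching player controller 0; a non-authority owner sends the world transform every Tick.
; A looping timer at a configurable frequency snapshots the pose, sending it by multicast from authority or to the server from clients.
; Non-owning receivers store the snapshot in ReplicatedPose.
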(event `self.ReceiveBeginPlay`
  (bind _fingerreplicationfrequency (`self.FingerReplicationFrequency`))
  ;[1 1 1] Set SkeletalMesh Reference and check for ownership
  (bind _asskeletal_mesh_component (cast `SkeletalMeshComponent` (`|GetArrayItem` (`self.GetChildrenComponents` true) 1)))
  (set `self.HandSkeleton` _asskeletal_mesh_component)
  (bind _output_get (set `self.IsOwner` (`self.HasOwnership`)))
  ;[1 1 1] Start hand replication execution loop
  (if (and _output_get (> _fingerreplicationfrequency 0))
    (`KismetSystemLibrary.K2_SetTimer` null "ReplicateFingers" (/ 1.0 (`KismetMathLibrary.Conv_IntToDouble` _fingerreplicationfrequency)) true)))

(event `ReplicateHandTransform`
  (params (SkeletalMesh :type "SkeletalMeshComponent Object Reference") (HandTransform :type "Transform Structure"))
  ;[1 1 1] Replicate Hand Transform on Server
  (`self.K2_SetWorldTransform` SkeletalMesh HandTransform false false))

(event `ReplicateFingersMulti`
  (params (Pose :type "PoseSnapshot Structure"))
  ;[1 1 1] Replicate Finger Pose on Server
  (if (not (`self.HasOwnership`))
    (set `self.ReplicatedPose` Pose)))

(event `self.ReceiveTick`
  (params (DeltaSeconds :type "Float (single-precision)"))
  ;[1 1 1] Replicate Hand Transform on Server
  (if (`self.IsOwner`)
    (`self.ReplicateHand`)))

(event `ReplicateFingersToServer`
  (params (Pose :type "PoseSnapshot Structure"))
  ;[1 1 1] Replicate Finger Pose on Server
  (if (not (`self.HasOwnership`))
    (set `self.ReplicatedPose` Pose)))

(fn `HasOwnership`
  (returns (IsOwner :type Boolean))
  (return (== (`Pawn.GetController` (`Actor.Instigator` (`self.GetOwner`))) (`GameplayStatics.GetPlayerController` 0))))

(fn `ReplicateFingers`
  (locals (PoseSnapshot :type "PoseSnapshot Structure"))
  (`SkeletalMeshComponent.SnapshotPose` (`self.HandSkeleton`) (`local.PoseSnapshot`))
  (if (`Actor.HasAuthority` (`self.GetOwner`))
    (`self.ReplicateFingersMulti` (`local.PoseSnapshot`))
    (else
      (`self.ReplicateFingersToServer` (`local.PoseSnapshot`)))))

(fn `ReplicateHand`
  (bind _handskeleton (`self.HandSkeleton`))
  (if (not (`Actor.HasAuthority` (`self.GetOwner`)))
    (`self.ReplicateHandTransform` _handskeleton (`self.K2_GetComponentToWorld` _handskeleton))))