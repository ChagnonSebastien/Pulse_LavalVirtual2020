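; Player pawn with motion-capture left and right hands, rackets, and a stop grid per hand marking a forward limit.
; BeginPlay gives each grid a dynamic material instance.
; Every tick, each grid follows its hand in Y and Z at a fixed X, and the remaining X distance, floored at zero, drives the material's Distance parameter.
; Each racket is hidden once its hand reaches or passes the grid plane.
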(event `self.ReceiveBeginPlay`
  ;[1 1 1] Set stop grid material to dynamic material
  (bind _returnvalue (`PrimitiveComponent.CreateDynamicMaterialInstance` (`self.Stop Grid L`) 0 "/Game/Assets/LimitGrid/Grid_Material.Grid_Material" "None"))
  (set `self.Grid Material L` _returnvalue)
  (bind _returnvalue_2 (`PrimitiveComponent.CreateDynamicMaterialInstance` (`self.Stop Grid R`) 0 "/Game/Assets/LimitGrid/Grid_Material.Grid_Material" "None"))
  (set `self.Grid Material R` _returnvalue_2)
  (`parent.ReceiveBeginPlay`))

(event `self.ReceiveTick`
  (params (DeltaSeconds :type "Float (single-precision)"))
  ;[1 1 1] Stop grid logic
  (bind _distance (`self.DistanceFromGrid` (`self.Stop Grid L`) (`self.MotionCaptureAvatar_L`)))
  (`MaterialInstanceDynamic.SetScalarParameterValue` (`self.Grid Material L`) "Distance" _distance)
  (`SceneComponent.SetVisibility` (`self.Racket_Blueprint_L`) (> _distance 0.0) false)
  (bind _distance_2 (`self.DistanceFromGrid` (`self.Stop Grid R`) (`self.MotionCaptureAvatar_R`)))
  (`MaterialInstanceDynamic.SetScalarParameterValue` (`self.Grid Material R`) "Distance" _distance_2)
  (`SceneComponent.SetVisibility` (`self.Racket_Blueprint_R`) (> _distance_2 0.0) false)
  (`parent.ReceiveTick` 0.0))

(fn `DistanceFromGrid`
  (params (StopGrid :type "StaticMeshComponent Object Reference") (Hand :type "MotionCaptureAvatarComponent Object Reference"))
  (returns (Distance :type "Float (double-precision)"))
  (`SceneComponent.K2_SetRelativeLocation` StopGrid (`KismetMathLibrary.MakeVector` (.x (`SceneComponent.RelativeLocation` StopGrid)) (.y (`SceneComponent.RelativeLocation` Hand)) (.z (`SceneComponent.RelativeLocation` Hand))) false false)
  (return (`KismetMathLibrary.FMax` (- (.x (`SceneComponent.RelativeLocation` StopGrid)) (.x (`SceneComponent.RelativeLocation` Hand))))))

(fn `UserConstructionScript`
  (`parent.UserConstructionScript`))