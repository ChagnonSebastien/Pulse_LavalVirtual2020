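; Countdown actor that shows a decreasing integer on two text components, Countdown1 and Countdown2.
; Tick feeds a one-second Delay, which ignores calls while pending and so acts as a roughly once-per-second timer.
; Each time it completes, CountdownValue drops by one while above zero and both texts update to the new value.
; Nothing further happens when the count reaches zero.
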(event `self.ReceiveTick`
  (params (DeltaSeconds :type "Float (single-precision)"))
  (`KismetSystemLibrary.Delay` 1.0)
  (if (< 0 (`self.countdown_value`))
    (set `self.countdown_value` (- (`self.countdown_value`) 1))
    (`TextRenderComponent.K2_SetText` (`self.Countdown1`) (`KismetTextLibrary.Conv_IntToText` (`self.countdown_value`)))
    (`TextRenderComponent.K2_SetText` (`self.Countdown2`) (`KismetTextLibrary.Conv_IntToText` (`self.countdown_value`)))))

(fn `UserConstructionScript`)